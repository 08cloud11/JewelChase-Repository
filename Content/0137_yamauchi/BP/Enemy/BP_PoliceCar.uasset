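; Police car Blueprint in the Enemy folder that destroys any actor tagged "Enemy" that begins overlapping it.
; The overlap event runs the parent's handler first, then validity-checks the other actor and tests its tag.
; BeginPlay and Tick are disabled stubs and the construction script only calls its parent, so this graph adds no other logic.
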(event `self.ReceiveActorBeginOverlap`
  (params (OtherActor :type "Actor Object Reference"))
  (`parent.ReceiveActorBeginOverlap` OtherActor)
  (if (`KismetSystemLibrary.IsValid` OtherActor)
    (if (`self.ActorHasTag` OtherActor "Enemy")
      (`self.K2_DestroyActor` OtherActor))))

(fn `UserConstructionScript`
  (`parent.UserConstructionScript`))