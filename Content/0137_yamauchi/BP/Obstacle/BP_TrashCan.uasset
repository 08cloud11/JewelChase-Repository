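; BP_TrashCan is a destructible obstacle that awards score and drops an item when destroyed by player bullets or an oil can.
; Each bullet overlap lowers Hp and briefly flashes the Mat_Color parameter on a dynamic material, which Tick resets after a short delay.
; Overlapping a BP_DestroyPoint removes it without reward, and every destruction spawns a particle effect.
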(event `self.ReceiveBeginPlay`
  (bind _returnvalue (`PrimitiveComponent.CreateDynamicMaterialInstance` (`self.StaticMesh`) 0 null "None"))
  (set `self.Mat_TrashCan` _returnvalue)
  (set `self.DefaultColorValue` (struct)))

(event `self.ReceiveTick`
  (params (DeltaSeconds :type "Float (single-precision)"))
  (if (!= (`self.ColorValue`) (`self.DefaultColorValue`))
    (bind _output_get (set `self.Time` (+ DeltaSeconds (`self.Time`))))
    (if (> _output_get 0.1)
      (set `self.Time` 0.0)
      (bind _output_get_2 (set `self.ColorValue` (`self.DefaultColorValue`)))
      (`MaterialInstanceDynamic.SetVectorParameterValue` (`self.Mat_TrashCan`) "Mat_Color" _output_get_2))))

(event `self.ReceiveActorBeginOverlap`
  (params (OtherActor :type "Actor Object Reference"))
  (`|ExecutionSequence`
    (:`then_0`
      (cast `/Game/0231_honma/BP/Stage/BP_DestroyPoint` OtherActor
        (:`then`
          (`self.K2_DestroyActor`))
        (:`CastFailed`
          (cast `/Game/0116_sakagami/BP/BP_PlayerBullet` OtherActor)
          (bind _output_get (set `self.Hp` (- (`self.Hp`) 1)))
          (if (<= _output_get 0)
            (bind _returnvalue (`GameplayStatics.GetActorOfClass` "/Game/0231_honma/BP/Stage/BP_ScoreManager.BP_ScoreManager_C"))
            (`ScoreManager.AddScore` _returnvalue (`self.Score`))
            (`self.SpawnDropItem`)
            (`self.K2_DestroyActor`)
            (else
              (set `self.ColorValue` (struct))
              (`MaterialInstanceDynamic.SetVectorParameterValue` :`self` (`self.Mat_TrashCan`) :`ParameterName` "Mat_Color"))))))
    (:`then_1`
      (cast `/Game/0137_yamauchi/BP/Obstacle/BP_OilCan` OtherActor)
      (bind _returnvalue_2 (`GameplayStatics.GetActorOfClass` "/Game/0231_honma/BP/Stage/BP_ScoreManager.BP_ScoreManager_C"))
      (`ScoreManager.AddScore` _returnvalue_2 (`self.Score`))
      (`self.SpawnDropItem`)
      (`self.K2_DestroyActor`))))

(event `self.ReceiveDestroyed`
  (`GameplayStatics.SpawnEmitterAtLocation` "/Game/0129_fukuda/Cascade/tramp_effect.tramp_effect" (`self.K2_GetActorLocation`) (struct) (3.0 3.0 3.0)))

(fn `UserConstructionScript`)