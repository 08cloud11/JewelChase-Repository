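; BP_OilCan is an explosive oil can obstacle that awards score when it blows up.
; A player bullet either detonates it or flashes its dynamic material orange, depending on an Hp check, with a Tick timer meant to restore the color.
; Detonation enables explosion collision, plays particles and sound, then destroys the actor.
; Overlapping another oil can also detonates it, allowing chain reactions, while destroy points remove it silently.
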(event `self.ReceiveBeginPlay`
  (bind _returnvalue (`PrimitiveComponent.CreateDynamicMaterialInstance` (`self.StaticMesh`) 0 null "None"))
  (set `self.Mat Obstacle` _returnvalue)
  (set `self.DefaultColorValue` (struct))
  (`SEManager.RegisterSE` (subsystem `SEManager`) "Boom" "/Game/0137_yamauchi/Sounds/Boom_Cue.Boom_Cue"))

(event `self.ReceiveTick`
  (params (DeltaSeconds :type "Float (single-precision)"))
  (if (!= (`self.ColorValue`) (`self.DefaultColorValue`))
    (bind _output_get (set `self.Time` (+ 0.0 (`self.Time`))))
    (if (> _output_get 0.1)
      (set `self.Time` 0.0)
      (bind _output_get_2 (set `self.ColorValue` (`self.DefaultColorValue`)))
      (`MaterialInstanceDynamic.SetVectorParameterValue` (`self.Mat Obstacle`) "Mat_Color" _output_get_2))))

(event `self.ReceiveActorBeginOverlap`
  (params (OtherActor :type "Actor Object Reference"))
  (cast `/Game/0231_honma/BP/Stage/BP_DestroyPoint` OtherActor
    (:`then`
      (`self.K2_DestroyActor`))
    (:`CastFailed`
      (cast `/Game/0116_sakagami/BP/BP_PlayerBullet` OtherActor
        (:`then`
          (if (<= 0 (`self.Hp`))
            (`self.TurnOnExplosionCollision`)
            (bind _returnvalue (`GameplayStatics.GetActorOfClass` "/Game/0231_honma/BP/Stage/BP_ScoreManager.BP_ScoreManager_C"))
            (`ScoreManager.AddScore` _returnvalue (`self.Score`))
            (`GameplayStatics.SpawnEmitterAtLocation` "/Game/0129_fukuda/Cascade/Booooom.Booooom" (`self.K2_GetActorLocation`) (struct) (3.0 3.0 3.0) :!label _label)
            (`SEManager.PlaySE2D` (subsystem `SEManager`) "Boom")
            (`self.K2_DestroyActor`)
            (else
              (bind _output_get (set `self.ColorValue` (struct :`R` 1.0 :`G` 0.082236 :`A` 1.0)))
              (`MaterialInstanceDynamic.SetVectorParameterValue` (`self.Mat Obstacle`) "Mat_Color" _output_get))))
        (:`CastFailed`
          (cast `/Game/0137_yamauchi/BP/Obstacle/BP_OilCan` OtherActor)
          (`self.TurnOnExplosionCollision`)
          (bind _returnvalue_2 (`GameplayStatics.GetActorOfClass` "/Game/0231_honma/BP/Stage/BP_ScoreManager.BP_ScoreManager_C"))
          (`ScoreManager.AddScore` _returnvalue_2 (`self.Score`))
          (goto _label))))))

(fn `UserConstructionScript`)