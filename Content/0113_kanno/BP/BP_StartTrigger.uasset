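; BP_StartTrigger plays the start-of-level intro through a referenced Level Sequence actor.
; BeginPlay waits briefly, passes a hard-wired true branch and a DoOnce, then starts the sequence player.
; Despite the trigger name, its overlap and Tick events are empty.
; A duplicate chain labeled as a click-to-start variant is disconnected and never runs.
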(event `self.ReceiveBeginPlay`
  ;[1 1 1] スタート時の演出
  (`KismetSystemLibrary.Delay` 1.5)
  (if true
    (`/Engine/EditorBlueprintResources/StandardMacros.DoOnce` false
      (:`Completed`
        (`MovieSceneSequencePlayer.Play` (`LevelSequenceActor.SequencePlayer` (`self.TargetLevelSequenceActor`)))))))

(event `self.CollisionComponent.OnComponentBeginOverlap`
  (params (OverlappedComponent :type "PrimitiveComponent Object Reference") (OtherActor :type "Actor Object Reference") (OtherComp :type "PrimitiveComponent Object Reference") (OtherBodyIndex :type Integer) (bFromSweep :type Boolean) (SweepResult :type "HitResult Structure (by ref)")))

(event `InputAction|Click`
  (params (Key :type "Key Structure"))
  ;[1 1 1] スタート時の演出（クリックしたらスタート）
)

(fn `UserConstructionScript`)