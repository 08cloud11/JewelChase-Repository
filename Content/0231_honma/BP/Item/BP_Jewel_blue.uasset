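; BP_Jewel_blue is a blue jewel pickup that awards score when the player character overlaps it.
; BeginPlay sets up a glowing blue dynamic material on its Sphere.
; Player overlap adds points and a jewel count to BP_ScoreManager, calls BgetON and raises emissive brightness; overlapping BP_DestroyPoint destroys the actor.
; An up-and-down bobbing routine exists but is unconnected, so it never runs.
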(event `self.ReceiveBeginPlay`
  (bind _returnvalue (`PrimitiveComponent.CreateDynamicMaterialInstance` (`self.Sphere`) 0 null "None"))
  (`MaterialInstanceDynamic.SetScalarParameterValue` _returnvalue "ScalarX" 0.0)
  (`MaterialInstanceDynamic.SetScalarParameterValue` _returnvalue "ScalarY" 0.5)
  (`MaterialInstanceDynamic.SetVectorParameterValue` _returnvalue "Mat_emiValue" (struct :`B` 1.0 :`A` 1.0))
  (`MaterialInstanceDynamic.SetScalarParameterValue` _returnvalue "JewelemiValue" 100.0))

(event `self.ReceiveTick`
  (params (DeltaSeconds :type "Float (single-precision)")))

(event `self.ReceiveActorBeginOverlap`
  (params (OtherActor :type "Actor Object Reference"))
  (cast `/Game/0231_honma/BP/Stage/BP_DestroyPoint` OtherActor
    (:`then`
      (`self.K2_DestroyActor`))
    (:`CastFailed`
      (cast `/Game/0116_sakagami/BP/BP_PlayerCharacter` OtherActor)
      (bind _returnvalue (`GameplayStatics.GetActorOfClass` "/Game/0231_honma/BP/Stage/BP_ScoreManager.BP_ScoreManager_C"))
      (`ScoreManager.AddScore` _returnvalue 500)
      (`ScoreManager.AddJewelNum` _returnvalue)
      (`self.bgetON`)
      (bind _returnvalue_2 (`PrimitiveComponent.CreateDynamicMaterialInstance` (`self.Sphere`) 0 null "None"))
      (`MaterialInstanceDynamic.SetScalarParameterValue` _returnvalue_2 "JewelemiValue" 200.0))))

(fn `UserConstructionScript`)