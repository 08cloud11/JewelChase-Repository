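; BP_Smog3 is a smog actor that changes the look of its Plane mesh according to its world X position.
; On BeginPlay it creates and stores a dynamic material instance for the plane.
; At start and on every Tick it sets that material's "Value" scalar parameter to the actor's X location, scaled down by a fixed divisor.
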(event `self.ReceiveBeginPlay`
  (bind _returnvalue_x (`KismetMathLibrary.BreakVector` (`self.K2_GetActorLocation`)))
  (bind _returnvalue (`PrimitiveComponent.CreateDynamicMaterialInstance` (`self.Plane`) 0 null "None"))
  (bind _output_get (set `self.SmogMat` _returnvalue))
  (`MaterialInstanceDynamic.SetScalarParameterValue` _output_get "Value" (/ (+ _returnvalue_x 0.0) 8000.0))
  (`MaterialInstanceDynamic.K2_GetScalarParameterValue` (`self.SmogMat`) "Value"))

(event `self.ReceiveTick`
  (params (DeltaSeconds :type "Float (single-precision)"))
  (bind _returnvalue_x (`KismetMathLibrary.BreakVector` (`self.K2_GetActorLocation`)))
  (`MaterialInstanceDynamic.SetScalarParameterValue` (`self.SmogMat`) "Value" (/ (+ _returnvalue_x 0.0) 8000.0))
  (`MaterialInstanceDynamic.K2_GetScalarParameterValue` (`self.SmogMat`) "Value"))

(fn `UserConstructionScript`)