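; Thrown playing-card (trump) actor in the stage select that flies toward a board and plays a hit sound on arrival.
; On its first Tick it gets a goal from BP_TrumpMng, then sets its direction and rotation.
; MoveX/Y/Z split a frame-rate-dependent step by Manhattan-normalized direction, with X always increasing and Z offset-biased.
; Hard-coded X/Z bounds stop movement and trigger the sound once; the actor destroys itself after three seconds.
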(event `self.ReceiveBeginPlay`
  (set `self.AfterSpawnTime` 0.0)
  (set `self.moveLength` 10.0)
  (set `self.moveDirection` (0.0 0.0 0.0))
  (set `self.BoardHit` false)
  (`SEManager.RegisterSE` (subsystem `SEManager`) "hit" (`self.HitSE`)))

(event `self.ReceiveTick`
  (params (DeltaSeconds :type "Float (single-precision)"))
  (bind (_returnvalue_x _returnvalue_y _returnvalue_z) (`KismetMathLibrary.BreakVector` (`self.K2_GetActorLocation`)))
  (`|ExecutionSequence`
    (:`then_0`
      (if (== (`self.moveDirection`) (0.0 0.0 0.0))
        (`self.TrumpInit`)))
    (:`then_1`
      (bind _output_get (set `self.AfterSpawnTime` (+ DeltaSeconds (`self.AfterSpawnTime`))))
      (if (< _output_get 3.0)
        (if (and (< _returnvalue_x 55.0) (> _returnvalue_z 75.0))
          (bind _returnvalue (`self.MoveX`))
          (bind _returnvalue_2 (`self.MoveY`))
          (bind _returnvalue_3 (`self.MoveZ`))
          (`self.K2_SetActorLocation` (`KismetMathLibrary.MakeVector` _returnvalue _returnvalue_2 _returnvalue_3))
          (elif (!= (`self.BoardHit`) true)
            (set `self.BoardHit` true)
            (`SEManager.PlaySE2D` (subsystem `SEManager`) "hit")))
        (else
          (`self.K2_DestroyActor`))))))

(event `TrumpInit`
  (bind (_movedirection_x _movedirection_y) (`KismetMathLibrary.BreakVector` (`self.moveDirection`)))
  (bind _returnvalue (`GameplayStatics.GetActorOfClass` "/Game/0231_honma/BP/StageSelect/BP_TrumpMng.BP_TrumpMng_C"))
  (bind _goallocation (`/Game/0231_honma/BP/StageSelect/BP_TrumpMng.ReturnGoalLocation` _returnvalue))
  (set `self.moveDirection` (- _goallocation (`self.K2_GetActorLocation`)))
  (`self.K2_SetActorRotation` (`KismetMathLibrary.MakeRotator` 0.0 135.0 (* _movedirection_y 0.45))))

(fn `MoveX`
  (returns (ReturnValue :type "Float (double-precision)"))
  (bind _returnvalue_x (`KismetMathLibrary.BreakVector` (`self.K2_GetActorLocation`)))
  (bind (_movedirection_x _movedirection_y _movedirection_z) (`KismetMathLibrary.BreakVector` (`self.moveDirection`)))
  (bind _returnvalue (`KismetMathLibrary.Abs` _movedirection_x))
  (return (+ _returnvalue_x (* (`self.moveLength`) (/ _returnvalue (+ _returnvalue (`KismetMathLibrary.Abs` _movedirection_y) (`KismetMathLibrary.Abs` _movedirection_z)))))))

(fn `MoveY`
  (returns (ReturnValue :type "Float (double-precision)"))
  (bind (_returnvalue_x _returnvalue_y) (`KismetMathLibrary.BreakVector` (`self.K2_GetActorLocation`)))
  (bind (_returnvalue_x_2 _returnvalue_y_2) (`KismetMathLibrary.BreakVector` (`self.K2_GetActorLocation`)))
  (bind (_movedirection_x _movedirection_y _movedirection_z) (`KismetMathLibrary.BreakVector` (`self.moveDirection`)))
  (bind (_movedirection_x_2 _movedirection_y_2) (`KismetMathLibrary.BreakVector` (`self.moveDirection`)))
  (bind (_movedirection_x_3 _movedirection_y_3 _movedirection_z_2) (`KismetMathLibrary.BreakVector` (`self.moveDirection`)))
  (bind _returnvalue (`KismetMathLibrary.Abs` _movedirection_y_3))
  (bind _returnvalue_2 (`KismetMathLibrary.Abs` _movedirection_y))
  (if (> _movedirection_y_2 0.0)
    (return (+ _returnvalue_y_2 (* (`self.moveLength`) (/ _returnvalue (+ (`KismetMathLibrary.Abs` _movedirection_x_3) _returnvalue (`KismetMathLibrary.Abs` _movedirection_z_2))))))
    (else
      (return (- _returnvalue_y (* (`self.moveLength`) (/ _returnvalue_2 (+ (`KismetMathLibrary.Abs` _movedirection_x) _returnvalue_2 (`KismetMathLibrary.Abs` _movedirection_z)))))))))

(fn `MoveZ`
  (returns (ReturnValue :type "Float (double-precision)"))
  (bind (_returnvalue_x _returnvalue_y _returnvalue_z) (`KismetMathLibrary.BreakVector` (`self.K2_GetActorLocation`)))
  (bind (_returnvalue_x_2 _returnvalue_y_2 _returnvalue_z_2) (`KismetMathLibrary.BreakVector` (`self.K2_GetActorLocation`)))
  (bind (_movedirection_x _movedirection_y _movedirection_z) (`KismetMathLibrary.BreakVector` (`self.moveDirection`)))
  (bind (_movedirection_x_2 _movedirection_y_2 _movedirection_z_2) (`KismetMathLibrary.BreakVector` (`self.moveDirection`)))
  (bind (_movedirection_x_3 _movedirection_y_3 _movedirection_z_3) (`KismetMathLibrary.BreakVector` (`self.moveDirection`)))
  (bind (_movedirection_x_4 _movedirection_y_4 _movedirection_z_4) (`KismetMathLibrary.BreakVector` (`self.moveDirection`)))
  (bind (_movedirection_x_5 _movedirection_y_5 _movedirection_z_5) (`KismetMathLibrary.BreakVector` (`self.moveDirection`)))
  (bind _returnvalue (`KismetMathLibrary.Abs` _movedirection_z))
  (bind _returnvalue_2 (`KismetMathLibrary.Abs` _movedirection_z_4))
  (if (> (- _movedirection_z_3 83.0) 0.0)
    (return (+ _returnvalue_z (* (`self.moveLength`) (/ _returnvalue_2 (+ (`KismetMathLibrary.Abs` _movedirection_x_4) (`KismetMathLibrary.Abs` _movedirection_y_4) _returnvalue_2)) (/ (- _movedirection_z_5 83.0) 3.0)) 0.0))
    (else
      (return (+ _returnvalue_z_2 (* (`self.moveLength`) (/ _returnvalue (+ (`KismetMathLibrary.Abs` _movedirection_x) (`KismetMathLibrary.Abs` _movedirection_y) _returnvalue)) (/ (- _movedirection_z_2 83.0) 3.0)))))))

(fn `UserConstructionScript`)