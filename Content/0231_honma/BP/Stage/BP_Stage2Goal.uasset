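; BP_Stage2Goal is the Stage 2 goal trigger, which saves the clear results and starts the transition to Master_Stage2_Goal when the player overlaps it.
; It loads or creates a BP_SaveGame in the "ranking" slot, inserts score, HP bonus, jewel bonus and stage number into ClearScore, then saves.
; A UI_Blackout widget receives the level name.
; A top-five ScoreUpdate helper exists but is never run.
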(event `Save`
  (`self.LoadGame`
    (:`output`
      (bind _returnvalue (`GameplayStatics.GetActorOfClass` "/Game/0231_honma/BP/Stage/BP_ScoreManager.BP_ScoreManager_C"))
      (bind _returnvalue_2 (`ScoreManager.Get_score` _returnvalue))
      (`self.ScoreSave` (`/Game/0231_honma/BP/BP_SaveGame.ClearScore` (`self.SaveData`)) _returnvalue_2
        (:`NewParam`
          (`self.SaveGame`))))))

(event `self.ReceiveActorBeginOverlap`
  (params (OtherActor :type "Actor Object Reference"))
  (castclass `/Game/0116_sakagami/BP/BP_PlayerCharacter` (`GameplayStatics.GetObjectClass` OtherActor))
  (`self.Save`)
  (bind _returnvalue (`|CreateWidget` "/Game/0231_honma/UI/Others/UI_Blackout.UI_Blackout_C"))
  (`UserWidget.AddToViewport` _returnvalue 0)
  (`BlackOut.SetOpenLevelName` _returnvalue "Master_Stage2_Goal"))

(fn `UserConstructionScript`)